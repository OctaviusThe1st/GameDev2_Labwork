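; BP_Trap_Disabler is an interactable pickup that disables a group of traps identified by TargetTrapIndex.
; On Interact it fires the TrapsDisabled dispatcher with that index, waits a tick, then destroys itself.
; The construction script colors its sphere red, blue or green by the index, and its interact state always reports false.
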(event EventInteract
  (params (NewParam :type Primitive%20Component%20Object%20Reference))
  (Default|CallTrapsDisabled (Variables|Default|GetTarget_trap_index))
  (Utilities|FlowControl|DelayUntilNextTick)
  (Actor|DestroyActor))

(fn ConstructionScript
  (Rendering|Material|SetMaterial (Variables|Default|GetSphere) 0 (Utilities|Select :Index (Variables|Default|GetTarget_trap_index) :Option%200 "/Game/materials/red.red" :Option%201 "/Game/materials/blue.blue" :Option%202 "/Game/materials/green.green")))

(fn GetInteractState
  (return false))