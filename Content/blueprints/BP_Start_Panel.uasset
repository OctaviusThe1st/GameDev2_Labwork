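; In-world start panel that lets the player pick a difficulty from 1 to 5 and start the game.
; Interact branches on the pressed object's name for plus, minus or start, then refreshes the panel's widget with the current difficulty.
; Start passes the difficulty to every platform cell, triggers the start gate, calls GameStart on the first-person character and stores the difficulty on it.
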(event EventInteract
  (params (NewParam :type Primitive%20Component%20Object%20Reference))
  (Utilities|FlowControl|Sequence
    (:then_0
      (switch string (Utilities|GetObjectName NewParam)
        (:Plus_Button
          (bind _result (Math|Integer|IncrementInt (Variables|Default|GetDifficulty))
            (:%20%20
              (if (> _result 5)
                (Variables|Default|SetDifficulty 5)))))
        (:Minus_Button
          (bind _result_2 (Math|Integer|DecrementInt (Variables|Default|GetDifficulty))
            (:%20%20
              (if (< _result_2 1)
                (Variables|Default|SetDifficulty 1)))))
        (:Start_Button
          (bind _outactors (Actor|GetAllActorsOfClass "/Game/blueprints/BP_Platfrom_Cell.BP_Platfrom_Cell_C"))
          (for _array_element _outactors
            (Default|Start _array_element (Variables|Default|GetDifficulty)))
          (bind _returnvalue (Actor|GetActorOfClass "/Game/blueprints/BP_Start_Gate.BP_Start_Gate_C"))
          (Default|Trigger _returnvalue)
          (bind _asbp_first_person_character (Utilities|Casting|CastToBP_FirstPersonCharacter (Game|GetPlayerCharacter 0)))
          (Default|GameStart _asbp_first_person_character)
          (Variables|/Game/FirstPerson/Blueprints/BP_FirstPersonCharacter.BP_FirstPersonCharacter_C|SetDifficulty_Ref _asbp_first_person_character (Variables|Default|GetDifficulty)))))
    (:then_1
      (Default|Update (Variables|Default|GetAs%20WBP%20Start%20Panel%20UI) (Variables|Default|GetDifficulty)))))

(event EventBeginPlay
  (bind _aswbp_start_panel_ui (Utilities|Casting|CastToWBP_Start_Panel_UI (UserInterface|GetUserWidgetObject (Variables|Default|GetWidget))))
  (bind _output_get (Variables|Default|SetAs%20WBP%20Start%20Panel%20UI _aswbp_start_panel_ui))
  (Default|Update _output_get 1))

(fn ConstructionScript)

(fn GetInteractState
  (return false))