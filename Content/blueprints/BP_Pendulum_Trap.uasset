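; Swinging pendulum blade trap, sized and oriented from its parent BP_Platfrom_Cell, that damages the player on contact.
; Trigger overlap plays a Swing timeline driving blade roll; a matching disabler event switches it off temporarily with a material change.
; The player's time-slow event lowers the trap's CustomTimeDilation.
; During a slowed swing, a second sword mesh appears and can be interacted with once, destroying it and calling the player's Gaze.
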(event Custom|Sword_hit
  (params (OverlappedComponent :type Primitive%20Component%20Object%20Reference) (OtherActor :type Actor%20Object%20Reference) (OtherComp :type Primitive%20Component%20Object%20Reference) (OtherBodyIndex :type Integer) (bFromSweep :type Boolean) (SweepResult :type Hit%20Result%20Structure%20%28by%20ref%29))
  (bind _as_bp_first_person_character (Variables|Default|GetAs%20BP%20First%20Person%20Character))
  ;[1 0.01979 0] Sword Hitbox
  (if (== OtherActor _as_bp_first_person_character)
    (Default|DamageFunction _as_bp_first_person_character (Variables|Default|GetSword_damage))))

(event Custom|OnComponentBeginOverlap_Event
  (params (OverlappedComponent :type Primitive%20Component%20Object%20Reference) (OtherActor :type Actor%20Object%20Reference) (OtherComp :type Primitive%20Component%20Object%20Reference) (OtherBodyIndex :type Integer) (bFromSweep :type Boolean) (SweepResult :type Hit%20Result%20Structure%20%28by%20ref%29))
  (bind _sworb1 (Variables|Default|Getsworb1))
  (bind _time_is_slowed (Variables|Default|GetTime_Is_Slowed))
  ;[0.9896 1 1] Trap Trigger
  (if (Variables|Default|GetIs_Enabled)
    (if (not (Variables|Default|GetTrap_active))
      (if (== OtherActor (Variables|Default|GetAs%20BP%20First%20Person%20Character))
        (bind _newtrack_0 (Timeline|Swing PlayFromStart)
          (:Update
            (Variables|Default|SetTrap_active true)
            (Transformation|SetRelativeRotation (Variables|Default|Getsworb) (Math|Rotator|MakeRotator (+ (* _newtrack_0 45.0) 0.0) 1.8e+02 (.yaw (Variables|/Game/blueprints/BP_Platfrom_Cell.BP_Platfrom_Cell_C|GetTrap_Rotation (Variables|Default|GetCell_Ref)))) false false))
          (:Finished
            (Variables|Default|SetTrap_active false)
            (Variables|Default|SetSword_Interactable false)))
        (if (Utilities|IsValid _sworb1)
          (Rendering|SetVisibility _sworb1 _time_is_slowed false)
          (Variables|Default|SetSword_Interactable _time_is_slowed))))))

(event Custom|Disabled
  (params (Trap_Target_Index :type Integer))
  ;[1 0.01049 0] Trap Disabled
  (if (== Trap_Target_Index 1)
    (Variables|Default|SetIs_Enabled false)
    (Rendering|Material|SetMaterial (Variables|Default|Getsworb) 0 "/Interchange/gltf/M_Default.M_Default")
    (Utilities|FlowControl|Delay 8.0)
    (Variables|Default|SetIs_Enabled true)
    (Rendering|Material|SetMaterial (Variables|Default|Getsworb) 0 "/Game/materials/blue.blue")))

(event Custom|Time_Slow
  (params (NewParam :type Boolean))
  ;[1 0.005718 0] Time Slow
  (bind _output_get (Variables|Default|SetTime_Is_Slowed NewParam))
  (if _output_get
    (Variables|Default|SetCustomTimeDilation 0.2)
    (else
      (Variables|Default|SetCustomTimeDilation 1.0))))

(event EventBeginPlay
  ;[0 1 0.03253] Begin Play Setup
  (bind _asbp_first_person_character (Utilities|Casting|CastToBP_FirstPersonCharacter (Game|GetPlayerCharacter 0)))
  (bind _output_get (Variables|Default|SetAs%20BP%20First%20Person%20Character _asbp_first_person_character))
  (EventDispatchers|BindEventtoTimeSlow _output_get (delegate Custom|Time_Slow))
  (Collision|AssignOnComponentBeginOverlap (Variables|Default|GetTrigger_box) (delegate Custom|OnComponentBeginOverlap_Event))
  (Collision|AssignOnComponentBeginOverlap (Variables|Default|GetSword_box) (delegate Custom|Sword_hit))
  (bind _outactors (Actor|GetAllActorsOfClass "/Game/blueprints/BP_Trap_Disabler.BP_Trap_Disabler_C"))
  (for _array_element _outactors
    (if (== (Variables|/Game/blueprints/BP_Trap_Disabler.BP_Trap_Disabler_C|GetTarget_trap_index _array_element) 1)
      (Variables|Default|SetDisabler_ref _array_element)))
  (EventDispatchers|BindEventtoTrapsDisabled (Variables|Default|GetDisabler_ref) (delegate Custom|Disabled)))

(event EventInteract
  (params (NewParam :type Primitive%20Component%20Object%20Reference))
  (if (Variables|Default|GetSword_Interactable)
    (Utilities|FlowControl|DoOnce false
      (:Completed
        (Components|DestroyComponent (Variables|Default|Getsworb1))
        (Default|Gaze (Variables|Default|GetAs%20BP%20First%20Person%20Character))))))

(fn ConstructionScript
  (bind _sworb (Variables|Default|Getsworb))
  (bind _trigger_box (Variables|Default|GetTrigger_box))
  (bind _asbp_platfrom_cell (Utilities|Casting|CastToBP_Platfrom_Cell (Actor|GetParentActor)))
  (bind _output_get (Variables|Default|SetCell_Ref _asbp_platfrom_cell))
  (Utilities|FlowControl|Sequence
    (:then_0
      (Transformation|SetRelativeLocation _sworb (Math|Vector|MakeVector 0.0 0.0 (+ (* (Variables|/Game/blueprints/BP_Platfrom_Cell.BP_Platfrom_Cell_C|Getwall_height _output_get) 1e+02) -2e+01)) false false)
      (Transformation|SetRelativeScale3D _sworb (Math|Conversions|ToVector(Float) (* (Variables|/Game/blueprints/BP_Platfrom_Cell.BP_Platfrom_Cell_C|Getwall_height _output_get) 0.05)))
      (Transformation|SetRelativeRotation _sworb (Math|Rotator|MakeRotator 45.0 (.pitch (Variables|/Game/blueprints/BP_Platfrom_Cell.BP_Platfrom_Cell_C|GetTrap_Rotation (Variables|Default|GetCell_Ref))) (.yaw (Variables|/Game/blueprints/BP_Platfrom_Cell.BP_Platfrom_Cell_C|GetTrap_Rotation (Variables|Default|GetCell_Ref)))) false false))
    (:then_1
      (Transformation|SetRelativeScale3D _trigger_box (Math|Vector|MakeVector (* (Variables|/Game/blueprints/BP_Platfrom_Cell.BP_Platfrom_Cell_C|GetGridSize (Variables|Default|GetCell_Ref)) 1.5) (* (Variables|/Game/blueprints/BP_Platfrom_Cell.BP_Platfrom_Cell_C|GetGridSize (Variables|Default|GetCell_Ref)) 1.5) (Variables|/Game/blueprints/BP_Platfrom_Cell.BP_Platfrom_Cell_C|Getwall_height (Variables|Default|GetCell_Ref))))
      (Transformation|SetRelativeLocation _trigger_box (Math|Vector|MakeVector 0.0 0.0 (* (Variables|/Game/blueprints/BP_Platfrom_Cell.BP_Platfrom_Cell_C|Getwall_height (Variables|Default|GetCell_Ref)) 5e+01)) false false))))

(fn GetInteractState
  (return false))